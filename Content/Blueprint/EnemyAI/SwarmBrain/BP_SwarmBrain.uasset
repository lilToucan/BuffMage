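; BP_SwarmBrain coordinates a swarm of enemies, deciding which active members attack and when.
; BindToEnemy subscribes to each enemy's activation events, which maintain the active list and start or stop a timeline used as an attack clock.
; When the clock finishes, it asks a clamped number of random active enemies to attack, retrying after delays on failure.
; Successful attackers move to the attacking list, and the clock restarts while active enemies remain.
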(event Custom|OnEnemyActivated_Event
  (params (Active%20enemy :type BP%20Base%20Enemy%20Object%20Reference))
  (Utilities|Array|RemoveItem (Variables|Default|GetAttackingEnemiesList) Active%20enemy)
  (Utilities|Array|AddUnique (Variables|Default|GetActiveEnemiesList) Active%20enemy)
  (if (not (Audio|Components|Audio|IsPlaying (Variables|Default|GetAttackClock)))
    (CallFunction|StartAttackClock)))

(event Custom|OnEnemyDeactivated_Event
  (params (Enemy :type BP%20Base%20Enemy%20Object%20Reference))
  (Utilities|Array|RemoveItem (Variables|Default|GetActiveEnemiesList) Enemy)
  (if (<= (Utilities|Array|Length (Variables|Default|GetActiveEnemiesList)) 0)
    (CallFunction|StopAttackClock)))

(event Custom|StartAttackClock
  (Components|Timeline|SetTimelineLength (Variables|Default|GetAttackClock) (Variables|Default|GetAttackTimer))
  (Timeline|AttackClock PlayFromStart
    (:Finished
      (if (> (Utilities|Array|Length (Variables|Default|GetActiveEnemiesList)) 0)
        (for _index (range 0 (- (Math|Integer|Clamp(Integer) (Variables|Default|GetNumberOfEnemiesAttacking) 1 (Utilities|Array|Length (Variables|Default|GetActiveEnemiesList))) 1))
          (bind (_outitem _outindex) (Utilities|Array|Random (Variables|Default|GetActiveEnemiesList) :!label _label))
          (Utilities|IsValid _outitem
            (:Is%20Valid
              (bind _canattack (Default|StartAttacking _outitem))
              (if _canattack
                (Utilities|Array|AddUnique (Variables|Default|GetAttackingEnemiesList) _outitem)
                (Utilities|Array|RemoveIndex (Variables|Default|GetActiveEnemiesList) _outindex)
                (else
                  (Utilities|FlowControl|Delay 0.2 :!label _label_2)
                  (goto _label))))
            (:Is%20Not%20Valid
              (Utilities|Array|RemoveIndex (Variables|Default|GetActiveEnemiesList) _outindex)
              (goto _label_2))))
        (if (> (Utilities|Array|Length (Variables|Default|GetActiveEnemiesList)) 0)
          (CallFunction|StartAttackClock))))))

(event Custom|StopAttackClock
  (Timeline|AttackClock Stop
    (:Finished
      (if (> (Utilities|Array|Length (Variables|Default|GetActiveEnemiesList)) 0)
        (for _index (range 0 (- (Math|Integer|Clamp(Integer) (Variables|Default|GetNumberOfEnemiesAttacking) 1 (Utilities|Array|Length (Variables|Default|GetActiveEnemiesList))) 1))
          (bind (_outitem _outindex) (Utilities|Array|Random (Variables|Default|GetActiveEnemiesList) :!label _label))
          (Utilities|IsValid _outitem
            (:Is%20Valid
              (bind _canattack (Default|StartAttacking _outitem))
              (if _canattack
                (Utilities|Array|AddUnique (Variables|Default|GetAttackingEnemiesList) _outitem)
                (Utilities|Array|RemoveIndex (Variables|Default|GetActiveEnemiesList) _outindex)
                (else
                  (Utilities|FlowControl|Delay 0.2 :!label _label_2)
                  (goto _label))))
            (:Is%20Not%20Valid
              (Utilities|Array|RemoveIndex (Variables|Default|GetActiveEnemiesList) _outindex)
              (goto _label_2))))
        (if (> (Utilities|Array|Length (Variables|Default|GetActiveEnemiesList)) 0)
          (CallFunction|StartAttackClock))))))

(event Custom|BindToEnemy
  (params (Enemy :type BP%20Base%20Enemy%20Object%20Reference))
  (EventDispatchers|BindEventtoOnSetActive Enemy (EventDispatchers|CreateEvent :!event Custom|OnEnemyActivated_Event))
  (EventDispatchers|BindEventtoOnSetInactive Enemy (EventDispatchers|CreateEvent :!event Custom|OnEnemyDeactivated_Event)))

(event EventBeginPlay
  (Components|Timeline|SetTimelineLength (Variables|Default|GetAttackClock) (Variables|Default|GetAttackTimer)))

(fn ConstructionScript)