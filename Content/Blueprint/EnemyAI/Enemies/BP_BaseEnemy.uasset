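; Base enemy character that runs a behavior tree through BP_EnemyController and mirrors its combat state into the Blackboard.
; On BeginPlay it writes attack and search settings to the Blackboard; stun, death and damage from BP_BuffMage or its projectiles update the stun, dead and Player keys.
; Hp and EnemyAttack events drive delayed HitStop and broadcast active, inactive and death dispatchers.
; Helper functions gate attacking on weapon reload and apply sphere-overlap damage.
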(event OnHit(Hp)
  (Variables|/Script/BuffMage.HitStopComponent|SetbShake (Variables|Default|GetHitStop) true)
  (Utilities|FlowControl|Delay 0.2)
  (Class|HitStopComponent|ActivateHitStun (Variables|Default|GetHitStop) 0.0))

(event OnAttackHitDel(EnemyAttack)
  (Variables|/Script/BuffMage.HitStopComponent|SetbShake (Variables|Default|GetHitStop) false)
  (Utilities|FlowControl|Delay 0.2)
  (Class|HitStopComponent|ActivateHitStun (Variables|Default|GetHitStop) 0.0))

(event OnDeathEnd(Hp)
  (Default|CallOnDeath self)
  (Components|DestroyComponent (Variables|Character|GetMesh))
  (Actor|DestroyActor))

(event OnDeathStarted(Hp)
  (Default|CallOnSetInactive self)
  (Development|PrintString "Set inactive Dead")
  (Components|Movement|StopMovementImmediately (Variables|Character|GetCharacterMovement))
  (AI|Components|Blackboard|SetValueasBool (AI|GetBlackboard 0) (Utilities|Name|MakeLiteralName "bIsDead") true))

(event OnStunned(Hp)
  (Default|CallOnSetInactive self)
  (Development|PrintString "Set inactive Stun"))

(event OnStunRecovered(Hp)
  (Default|CallOnSetActive self)
  (Development|PrintString "Set active Stun"))

(event Custom|Stunned_Event
  (if (not (ScalableFloat|GetValueasBool (Variables|Default|GetBlackBoard) (Utilities|Name|MakeLiteralName "bIsStunned")))
    (AI|Components|Blackboard|SetValueasBool (Variables|Default|GetBlackBoard) (Utilities|Name|MakeLiteralName "bIsStunned") true)))

(event Custom|StunRecovery_Event
  (AI|Components|Blackboard|SetValueasBool (Variables|Default|GetBlackBoard) (Utilities|Name|MakeLiteralName "bIsStunned") false))

(event Custom|OnAttackStarted_Event
  (Default|CallOnSetInactive self)
  (Development|PrintString "Set inactive Attack"))

(event Custom|OnAttackEnded_Event
  (Default|CallOnSetActive self)
  (Development|PrintString "Set active Attack"))

(event EventBeginPlay
  (Utilities|FlowControl|Sequence
    (:then_0
      (bind _asbp_enemy_controller (Utilities|Casting|CastToBP_EnemyController (Pawn|GetController)))
      (Default|SetBehaviorTree _asbp_enemy_controller (Variables|BehaviorTree|GetBTAsset))
      (bind _output_get (Variables|Default|SetBlackBoard (AI|GetBlackboard _asbp_enemy_controller)))
      (Variables|/Game/Blueprint/ActorComponents/BP_EnemyAttack.BP_EnemyAttack_C|SetBlackboard (Variables|Default|GetEnemyAttack) _output_get))
    (:then_1
      (EventDispatchers|BindEventtoOnStunned (Variables|Default|GetHp) (EventDispatchers|CreateEvent :!event Custom|Stunned_Event))
      (EventDispatchers|BindEventtoOnStunRecovered (Variables|Default|GetHp) (EventDispatchers|CreateEvent :!event Custom|StunRecovery_Event)))
    (:then_2
      (AI|Components|Blackboard|SetValueasFloat (AI|GetBlackboard 0) (Utilities|Name|MakeLiteralName "AttackDistance") (Variables|BehaviorTree|GetAttackDistance))
      (AI|Components|Blackboard|SetValueasFloat (AI|GetBlackboard 0) (Utilities|Name|MakeLiteralName "SearchRadious") (Variables|BehaviorTree|GetSearchRadious))
      (AI|Components|Blackboard|SetValueasFloat (AI|GetBlackboard 0) (Utilities|Name|MakeLiteralName "SearchConeAngle") (Variables|BehaviorTree|GetSearchConeAngle)))
    (:then_3
      (EventDispatchers|BindEventtoOnAttackStart (Variables|Default|GetEnemyAttack) (EventDispatchers|CreateEvent :!event Custom|OnAttackStarted_Event))
      (EventDispatchers|BindEventtoOnAttackEnded (Variables|Default|GetEnemyAttack) (EventDispatchers|CreateEvent :!event Custom|OnAttackEnded_Event)))))

(event Collision|EventActorBeginOverlap
  (params (OtherActor :type Actor%20Object%20Reference)))

(event EventTick
  (params (DeltaSeconds :type Float%20%28single-precision%29)))

(event Game|Damage|EventAnyDamage
  (params (Damage :type Float%20%28single-precision%29) (DamageType :type Damage%20Type%20Object%20Reference) (InstigatedBy :type Controller%20Object%20Reference) (DamageCauser :type Actor%20Object%20Reference))
  (bind _asbp_buff_mage (Utilities|Casting|CastToBP_BuffMage DamageCauser)
    (:then
      (CallFunction|SetPlayerVar _asbp_buff_mage))
    (:CastFailed
      (bind _asbp_projectile (Utilities|Casting|CastToBP_Projectile DamageCauser))
      (bind _asbp_buff_mage_2 (Utilities|Casting|CastToBP_BuffMage (Variables|/Game/Blueprint/Projectiles/BP_Projectile.BP_Projectile_C|GetShooter _asbp_projectile)))
      (AI|Components|Blackboard|SetValueasObject (Variables|Default|GetBlackBoard) (Utilities|Name|MakeLiteralName "Player") _asbp_buff_mage_2))))

(fn ConstructionScript
  (Variables|/Script/BuffMage.HitStopComponent|SetSceneComponent (Variables|Default|GetHitStop) (Variables|Character|GetMesh)))

(fn AttackSequenceFunction
  (params (SphereRadius :type Float%20%28single-precision%29))
  (bind _outactors (Collision|SphereOverlapActors (Transformation|GetWorldLocation (Variables|Default|GetAttackOverlapPoint)) SphereRadius (Utilities|Array|MakeArray "ObjectTypeQuery3") 0 (Utilities|Array|MakeArray self)))
  (for _array_element _outactors
    (Game|Damage|ApplyDamage _array_element 1.0 0 0)))

(fn StartAttacking
  (if (not (Utilities|Struct|BreakDynamicWeaponData (Variables|/Script/BuffMage.AttackComponent|GetCurrentWeapon (Variables|Default|GetEnemyAttack))))
    (AI|Components|Blackboard|SetValueasBool (Variables|Default|GetBlackBoard) (Utilities|Name|MakeLiteralName "bCanAttack") true)
    (return true)
    (else
      (return false))))

(fn SetPlayerVar
  (params (Player :type Object%20Object%20Reference))
  (AI|Components|Blackboard|SetValueasObject (Variables|Default|GetBlackBoard) (Utilities|Name|MakeLiteralName "Player") Player))