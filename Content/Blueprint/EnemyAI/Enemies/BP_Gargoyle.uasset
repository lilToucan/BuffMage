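; BP_Gargoyle is an enemy Blueprint that joins the game's melee swarm AI with randomized positioning parameters.
; On BeginPlay it rolls an EQS point count and radius, then derives point spacing from the circumference plus a small padding.
; It writes all three values to its Blackboard, then registers itself with the MeleeSwarmBrain on GM_BuffMage.
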(event EventBeginPlay
  (|CallParentFunction)
  (Utilities|FlowControl|Sequence
    (:then_0
      (Variables|Eqs|SetPointsEqs (Math|Random|RandomIntegerinRange (Variables|Eqs|GetMinPointsEqs) (Variables|Eqs|GetMaxPointsEqs)))
      (Variables|Eqs|SetRangeEqs (Math|Random|RandomFloatinRange (Variables|Eqs|GetMixRangeEqs) (Variables|Eqs|GetMaxRangeEqs)))
      (Variables|Eqs|SetDistanceBetweenPointsEqs (+ (/ (* (Variables|Eqs|GetRangeEqs) 2.0 (Math|Trig|GetPI)) (Math|Conversions|ToFloat(Integer) (Variables|Eqs|GetPointsEqs))) 1e+01)))
    (:then_1
      (AI|Components|Blackboard|SetValueasFloat (Variables|Default|GetBlackBoard) (Utilities|Name|MakeLiteralName "RangeEqs") (Variables|Eqs|GetRangeEqs))
      (Class|BlackboardComponent|SetValueasInt (Variables|Default|GetBlackBoard) (Utilities|Name|MakeLiteralName "PointsEqs") (Variables|Eqs|GetPointsEqs))
      (AI|Components|Blackboard|SetValueasFloat (Variables|Default|GetBlackBoard) (Utilities|Name|MakeLiteralName "DistanceBetweenPointsEqs") (Variables|Eqs|GetDistanceBetweenPointsEqs)))
    (:then_2
      (bind _asgm_buff_mage (Utilities|Casting|CastToGM_BuffMage (Game|GetGameMode)))
      (Default|BindTOEnemy (Variables|/Game/Blueprint/Core/GameModes/GM_BuffMage.GM_BuffMage_C|GetMeleeSwarmBrain _asgm_buff_mage) self))))

(event Collision|EventActorBeginOverlap
  (params (OtherActor :type Actor%20Object%20Reference))
  (|CallParentFunction OtherActor) ; This node is disabled and will not be called.\nDrag off pins to build functionality.
)

(event EventTick
  (params (DeltaSeconds :type Float%20%28single-precision%29))
  (|CallParentFunction DeltaSeconds) ; This node is disabled and will not be called.\nDrag off pins to build functionality.
)

(fn ConstructionScript
  (|CallParentFunction))