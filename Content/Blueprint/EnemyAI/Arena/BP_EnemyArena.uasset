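; Enemy arena that locks the BP_BuffMage player in and runs successive waves of skeletons and gargoyles.
; Entering the trigger closes linked doors, disables actor collision and spawns the first wave at actor-relative positions.
; Enemy death events decrement an alive count, starting the next wave at zero and reopening doors once waves run out.
; The construction script previews spawn points as debug capsules colored by enemy type.
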(event OnComponentBeginOverlap(Trigger)
  (params (OverlappedComponent :type Primitive%20Component%20Object%20Reference) (OtherActor :type Actor%20Object%20Reference) (OtherComp :type Primitive%20Component%20Object%20Reference) (OtherBodyIndex :type Integer) (bFromSweep :type Boolean) (SweepResult :type Hit%20Result%20Structure%20%28by%20ref%29))
  (Utilities|Casting|CastToBP_BuffMage OtherActor)
  (bind _array_element (Utilities|Array|ForEachLoopwithBreak (Variables|Default|GetDoorsToClose))
    (:LoopBody
      (Default|ClosetheDoor _array_element))
    (:Completed
      (CallFunction|StartNextWave (Variables|Default|GetAs%20BP%20Buff%20Mage))
      (Collision|SetActorEnableCollision false))))

(event Custom|StartNextWave
  (params (BuffMage :type BP%20Buff%20Mage%20Object%20Reference))
  (if (>= (Variables|Default|GetCurrentWave) (Utilities|Array|Length (Variables|Default|GetWaves)))
    (CallFunction|ArenaOver)
    (else
      (bind _array_element (Utilities|Array|ForEachLoopwithBreak (Utilities|Struct|BreakWave (Utilities|Array|Get(acopy) (Variables|Default|GetWaves) (Variables|Default|GetCurrentWave))))
        (:LoopBody
          (for _array_element_2 (.EnemyPositions (Utilities|Struct|BreakWaveData _array_element))
            (switch Utilities|FlowControl|Switch|SwitchonEEnemyType (.EnemyType (Utilities|Struct|BreakWaveData _array_element))
              (:SkeletonMelee
                _)
              (:SkeletonRanged
                _)
              (:Gargoyle
                _))
            (bind _returnvalue (Game|SpawnActorfromClass (|SelectEnemyClass (.EnemyType (Utilities|Struct|BreakWaveData _array_element))) (Math|Transform|MakeTransform (+ _array_element_2 (Transformation|GetActorLocation)) "0, 0, 0" "1.000000,1.000000,1.000000") "Undefined" "MultiplyWithRoot" 0 0))
            (bind _asbp_base_enemy (Utilities|Casting|CastToBP_BaseEnemy _returnvalue))
            (Default|SetPlayerVar _asbp_base_enemy BuffMage)
            (Math|Integer|IncrementInt (Variables|Default|GetAliveEnemies)
              (:%20%20
                (EventDispatchers|BindEventtoOnDeath _asbp_base_enemy (EventDispatchers|CreateEvent :!event Custom|OnEnemyDeath_Event))))))
        (:Completed
          (Math|Integer|IncrementInt (Variables|Default|GetCurrentWave)))))))

(event Custom|OnEnemyDeath_Event
  (params (Enemy :type BP%20Base%20Enemy%20Object%20Reference))
  (EventDispatchers|UnbindEventfromOnDeath Enemy (EventDispatchers|CreateEvent :!event Custom|OnEnemyDeath_Event))
  (bind _result (Math|Integer|DecrementInt (Variables|Default|GetAliveEnemies))
    (:%20%20
      (if (<= _result 0)
        (CallFunction|StartNextWave (Variables|Default|GetAs%20BP%20Buff%20Mage))))))

(event Custom|ArenaOver
  (bind _array_element (Utilities|Array|ForEachLoopwithBreak (Variables|Default|GetDoorsToClose))
    (:LoopBody
      (Default|OpentheDoor _array_element))))

(event EventBeginPlay
  (bind _asbp_buff_mage (Utilities|Casting|CastToBP_BuffMage (Game|Player|GetPlayerPawn 0)))
  (Variables|Default|SetAs%20BP%20Buff%20Mage _asbp_buff_mage))

(fn ConstructionScript
  (bind _returnvalue (Math|Float|MakeLiteralFloat 88.0))
  (Rendering|Debug|FlushPersistentDebugLines)
  (for _array_element (Variables|Default|GetWaves)
    (bind _array_element_2 (Utilities|Array|ForEachLoopwithBreak (Utilities|Struct|BreakWave _array_element))
      (:LoopBody
        (for _array_element_3 (.EnemyPositions (Utilities|Struct|BreakWaveData _array_element_2))
          (Rendering|Debug|DrawDebugCapsule (+ (+ _array_element_3 (Transformation|GetActorLocation)) (* "0.000000,0.000000,1.000000" _returnvalue)) _returnvalue 34.0 "0, 0, 0" (Utilities|Select :Index (.EnemyType (Utilities|Struct|BreakWaveData _array_element_2)) :none (Math|Color|MakeColor 0.0 0.0 0.0) :SkeletonMelee "(R=0.850999,G=1.000000,B=0.044343,A=1.000000)" :SkeletonRanged "(R=0.000000,G=1.000000,B=0.147272,A=1.000000)" :Gargoyle "(R=1.000000,G=0.346225,B=0.005148,A=1.000000)") 1e+18 0.0))))))