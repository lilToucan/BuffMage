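; An arena door Blueprint that slides open and closed in response to its Lock component.
; Lock's unlocked and locked events play or reverse-from-end a timeline that lerps the Door's relative location between the Closed and Open marker positions.
; Duration sets the timeline play rate, reapplied on begin play, before each move and whenever SetDuration changes it.
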(event OnLocked(Lock)
  (CallFunction|ClosetheDoor))

(event OnUnLocked(Lock)
  (CallFunction|OpentheDoor))

(event Custom|OpenTheDoor
  (CallFunction|ApplyPlayRate)
  (bind _opendoor (Timeline|OpenDoor Play)
    (:Update
      (Transformation|SetRelativeLocation (Variables|Default|GetDoor) (Math|Vector|Lerp(Vector) (Variables|/Script/Engine.SceneComponent|GetRelativeLocation (Variables|Default|GetClosed)) (Variables|/Script/Engine.SceneComponent|GetRelativeLocation (Variables|Default|GetOpen)) _opendoor) false false))))

(event Custom|CloseTheDoor
  (CallFunction|ApplyPlayRate)
  (bind _opendoor (Timeline|OpenDoor ReverseFromEnd)
    (:Update
      (Transformation|SetRelativeLocation (Variables|Default|GetDoor) (Math|Vector|Lerp(Vector) (Variables|/Script/Engine.SceneComponent|GetRelativeLocation (Variables|Default|GetClosed)) (Variables|/Script/Engine.SceneComponent|GetRelativeLocation (Variables|Default|GetOpen)) _opendoor) false false))))

(event EventBeginPlay
  (Variables|Default|SetStartRelativeLocation (Variables|/Script/Engine.SceneComponent|GetRelativeLocation (Variables|Default|GetDoor)))
  (CallFunction|ApplyPlayRate))

(fn ConstructionScript)

(fn ApplyPlayRate
  (Components|Timeline|SetPlayRate (Variables|Default|GetOpenDoor) (/ 1.0 (Variables|Default|GetDuration))))

(fn SetDuration
  (params (NewDuration :type Float%20%28double-precision%29))
  (Variables|Default|SetDuration NewDuration)
  (CallFunction|ApplyPlayRate))