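; Anim notify state that runs continuous capsule hit detection between two weapon or body sockets during an attack animation.
; On begin it reduces ammo through the owner's AttackComponent.
; Each tick it writes half the socket distance to the current weapon's HalfHeight, then calls HitDetection at the midpoint using the start socket's rotation.
; Without an AttackComponent, it draws debug spheres and a cylinder at the sockets instead.
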(fn ReceivedNotifyBegin
  (params (MeshComp :type Skeletal%20Mesh%20Component%20Object%20Reference) (Animation :type Anim%20Sequence%20Base%20Object%20Reference) (TotalDuration :type Float%20%28single-precision%29) (EventReference :type Anim%20Notify%20Event%20Reference%20Structure%20%28by%20ref%29))
  (bind _returnvalue (Components|GetOwner MeshComp))
  (bind _returnvalue_2 (Actor|GetComponentbyClass _returnvalue "/Script/BuffMage.AttackComponent"))
  (Utilities|IsValid _returnvalue_2
    (:Is%20Valid
      (Class|AttackComponent|ReduceAmmo _returnvalue_2)
      (return true))))

(fn ReceivedNotifyTick
  (params (MeshComp :type Skeletal%20Mesh%20Component%20Object%20Reference) (Animation :type Anim%20Sequence%20Base%20Object%20Reference) (FrameDeltaTime :type Float%20%28single-precision%29) (EventReference :type Anim%20Notify%20Event%20Reference%20Structure%20%28by%20ref%29))
  (LocalVariables|SetMesh MeshComp)
  (bind _output_get (LocalVariables|SetAttackComp (Actor|GetComponentbyClass (Components|GetOwner (LocalVariables|GetMesh)) "/Script/BuffMage.AttackComponent")))
  (Utilities|IsValid _output_get
    (:Is%20Valid
      (Variables|/Script/BuffMage.WeaponDataAsset|SetHalfHeight (Utilities|Struct|BreakDynamicWeaponData (Variables|/Script/BuffMage.AttackComponent|GetCurrentWeapon (LocalVariables|GetAttackComp))) (CallFunction|GetCapsuleHalfHight (LocalVariables|GetMesh)))
      (Class|AttackComponent|HitDetection (LocalVariables|GetAttackComp) (Variables|Default|GetEndAttackSocketName) (Math|Vector|Lerp(Vector) (Transformation|GetSocketLocation (LocalVariables|GetMesh) (Variables|Default|GetStartAttackSocketName)) (Transformation|GetSocketLocation (LocalVariables|GetMesh) (Variables|Default|GetEndAttackSocketName)) 0.5) (Transformation|GetSocketRotation (LocalVariables|GetMesh) (Variables|Default|GetStartAttackSocketName)))
      (return true))
    (:Is%20Not%20Valid
      (Rendering|Debug|DrawDebugSphere (LocalVariables|GetMesh) (Transformation|GetSocketLocation (LocalVariables|GetMesh) (Variables|Default|GetStartAttackSocketName)) 1e+01 12 "(R=0.842885,G=0.000000,B=0.000000,A=1.000000)")
      (Rendering|Debug|DrawDebugSphere (LocalVariables|GetMesh) (Transformation|GetSocketLocation (LocalVariables|GetMesh) (Variables|Default|GetEndAttackSocketName)) 1e+01 12 "(R=0.629483,G=0.480443,B=1.000000,A=1.000000)")
      (Class|KismetSystemLibrary|DrawDebugCylinder (LocalVariables|GetMesh) (Transformation|GetSocketLocation (LocalVariables|GetMesh) (Variables|Default|GetStartAttackSocketName)) (Transformation|GetSocketLocation (LocalVariables|GetMesh) (Variables|Default|GetEndAttackSocketName)) 2e+01 12 "(R=1.000000,G=0.543111,B=0.639118,A=1.000000)" 1.0 0.0)
      (return true))))

(fn GetCapsuleHalfHight
  (params (Mesh :type Scene%20Component%20Object%20Reference))
  (return (/ (Math|Vector|Distance(Vector) (Transformation|GetSocketLocation Mesh (Variables|Default|GetStartAttackSocketName)) (Transformation|GetSocketLocation Mesh (Variables|Default|GetEndAttackSocketName))) 2.0)))