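; Anim notify that plays a randomly chosen sound in 3D at the animated mesh's owning actor.
; When fired, it picks an entry from its Sounds array and plays it at the owner's location, doing nothing if the array is empty.
; Pitch is randomized within a configurable min/max range, while volume and start time come from the notify's variables.
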(fn ReceivedNotify
  (params (MeshComp :type Skeletal%20Mesh%20Component%20Object%20Reference) (Animation :type Anim%20Sequence%20Base%20Object%20Reference) (EventReference :type Anim%20Notify%20Event%20Reference%20Structure%20%28by%20ref%29))
  (if (> (Utilities|Array|Length (Variables|Default|GetSounds)) 0)
    (LocalVariables|SetOwner (Components|GetOwner MeshComp))
    (Audio|PlaySoundatLocation (.OutItem (Utilities|Array|Random (Variables|Default|GetSounds))) (Transformation|GetActorLocation (LocalVariables|GetOwner)) "0, 0, 0" (Variables|Default|GetVolume%20Multiplier) (Math|Random|RandomFloatinRange (Variables|Default|GetMinPitchMult) (Variables|Default|GetMaxPitchMult)) (Variables|Default|GetStart%20Time) 0 0 0 0)
    (return true)))