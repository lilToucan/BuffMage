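; ANS_ContinuousAttack is an anim notify state that runs a continuous attack over a span of an animation.
; On begin it calls ReduceAmmo once on the owner's AttackComponent.
; Each tick it calls that component's HitDetection with the configured attack socket name.
; When the owner has no AttackComponent, the tick draws a debug sphere in the notify color instead.
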(fn ReceivedNotifyBegin
  (params (MeshComp :type Skeletal%20Mesh%20Component%20Object%20Reference) (Animation :type Anim%20Sequence%20Base%20Object%20Reference) (TotalDuration :type Float%20%28single-precision%29) (EventReference :type Anim%20Notify%20Event%20Reference%20Structure%20%28by%20ref%29))
  (bind _returnvalue (Components|GetOwner MeshComp))
  (bind _returnvalue_2 (Actor|GetComponentbyClass _returnvalue "/Script/BuffMage.AttackComponent"))
  (Utilities|IsValid _returnvalue_2
    (:Is%20Valid
      (Class|AttackComponent|ReduceAmmo _returnvalue_2)
      (return true))))

(fn ReceivedNotifyTick
  (params (MeshComp :type Skeletal%20Mesh%20Component%20Object%20Reference) (Animation :type Anim%20Sequence%20Base%20Object%20Reference) (FrameDeltaTime :type Float%20%28single-precision%29) (EventReference :type Anim%20Notify%20Event%20Reference%20Structure%20%28by%20ref%29))
  (bind _returnvalue (Components|GetOwner MeshComp))
  (bind _returnvalue_2 (Actor|GetComponentbyClass _returnvalue "/Script/BuffMage.AttackComponent"))
  (Utilities|IsValid _returnvalue_2
    (:Is%20Valid
      (Class|AttackComponent|HitDetection _returnvalue_2 (Variables|Default|GetAttackSocketName))
      (return true))
    (:Is%20Not%20Valid
      (Rendering|Debug|DrawDebugSphere MeshComp "0, 0, 0" 1e+02 12 (Math|Conversions|ToLinearColor(Color) (Variables|Default|GetNotifyColor)))
      (return true))))