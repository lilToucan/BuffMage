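; BP_Projectile is a pooled projectile actor that flies straight and damages what it overlaps.
; Activate stores its stats and shooter, places it, and enables tick, visibility and collision.
; Tick moves it forward by Velocity each frame, without sweep or delta-time scaling; ExplosionRange is stored but unused.
; Overlaps ignore the shooter and same-class actors; others take damage, then Deactivate disables it and returns it to the ObjectPoolingSubsystem.
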(event EventBeginPlay)

(event EventTick
  (params (DeltaSeconds :type Float%20%28single-precision%29))
  (Transformation|SetActorLocation (+ (Transformation|GetActorLocation) (* (Transformation|GetActorForwardVector) (Variables|Default|GetVelocity))) false false))

(event EventActivate
  (params (Velocity :type Float%20%28single-precision%29) (Damage :type Float%20%28single-precision%29) (ExplosionRange :type Float%20%28single-precision%29) (Shooter :type Actor%20Object%20Reference) (Position :type Vector :default "0, 0, 0") (Rotation :type Rotator :default "0, 0, 0"))
  (Variables|Default|SetVelocity Velocity)
  (Variables|Default|SetDamage Damage)
  (Variables|Default|SetExplosion%20Range ExplosionRange)
  (Variables|Default|SetShooter Shooter)
  (Transformation|SetActorLocation Position false false)
  (Transformation|SetActorRotation Rotation)
  (Actor|Tick|SetActorTickEnabled true)
  (Rendering|SetActorHiddenInGame false)
  (Collision|SetActorEnableCollision true))

(event EventDeactivate
  (Rendering|SetActorHiddenInGame true)
  (Collision|SetActorEnableCollision false)
  (Actor|Tick|SetActorTickEnabled false)
  (Class|ObjectPoolingSubsystem|ReturnActortoPool (Subsystems|GetObjectPoolingSubsystem) (Utilities|GetClass self) self))

(event Collision|EventActorBeginOverlap
  (params (OtherActor :type Actor%20Object%20Reference))
  (if (not (or (== (Utilities|GetClass OtherActor) (Utilities|GetClass self)) (== OtherActor (Variables|Default|GetShooter))))
    (Game|Damage|ApplyDamage OtherActor (Variables|Default|GetDamage) 0 self)
    (Class|ProjectilePoolable|Deactivate self)))

(fn ConstructionScript)