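; Testing dummy actor that patrols a list of waypoints and destroys itself after enough damage events.
; BeginPlay appends its spawn location and swaps it into index 0, then starts a self-restarting timeline that lerps it between points.
; At the last point the route reverses, and later reverse moves step back two indices at a time.
; Any damage, whatever the amount, decrements HP by one.
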(event Custom|PlayTimelineFromStart
  (if (and (< (Variables|Default|GetWaypointIndex) (- (Utilities|Array|Length (Variables|Default|GetWaypoints)) 1)) (not (Variables|Default|GetIsReverse)))
    (Math|Integer|IncrementInt (Variables|Default|GetWaypointIndex)
      (:%20%20
        _))
    (else
      (if (Variables|Default|GetIsReverse)
        (Variables|Default|SetWaypointIndex (- (Variables|Default|GetWaypointIndex) 2))
        (else
          (Variables|Default|SetIsReverse true)
          (Math|Integer|DecrementInt (Variables|Default|GetWaypointIndex)
            (:%20%20
              _))))
      (if (> (Variables|Default|GetWaypointIndex) 0)
        _
        (else
          (Variables|Default|SetIsReverse false)))))
  (Variables|Default|SetStartPos (Transformation|GetActorLocation))
  (Variables|Default|SetEndPos (Utilities|Array|Get(acopy) (Variables|Default|GetWaypoints) (Variables|Default|GetWaypointIndex)))
  (bind _fiveseconds (Timeline|Waypoint PlayFromStart)
    (:Update
      (Transformation|SetActorLocation (Math|Vector|Lerp(Vector) (Variables|Default|GetStartPos) (Variables|Default|GetEndPos) _fiveseconds) false false))
    (:Finished
      (CallFunction|PlayTimelinefromStart))))

(event EventBeginPlay
  (bind _returnvalue (Utilities|Array|Add (Variables|Default|GetWaypoints) (Transformation|GetActorLocation)))
  (Utilities|Array|Swap (Variables|Default|GetWaypoints) _returnvalue)
  (CallFunction|PlayTimelinefromStart))

(event Collision|EventActorBeginOverlap
  (params (OtherActor :type Actor%20Object%20Reference)))

(event EventTick
  (params (DeltaSeconds :type Float%20%28single-precision%29)))

(event Game|Damage|EventAnyDamage
  (params (Damage :type Float%20%28single-precision%29) (DamageType :type Damage%20Type%20Object%20Reference) (InstigatedBy :type Controller%20Object%20Reference) (DamageCauser :type Actor%20Object%20Reference))
  (bind _result (Math|Integer|DecrementInt (Variables|Default|GetHP))
    (:%20%20
      (if (<= _result 0)
        (Actor|DestroyActor)))))

(fn ConstructionScript)