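; BP_HidingEnemy is an AI enemy Blueprint that joins the game mode's ranged swarm.
; On BeginPlay it runs the parent logic, casts the game mode to GM_BuffMage and binds itself to that mode's RangedSwarmBrain.
; It defines no hiding behavior of its own: tick and overlap events are disabled, and the construction script only calls the parent.
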(event EventBeginPlay
  (|CallParentFunction)
  (bind _asgm_buff_mage (Utilities|Casting|CastToGM_BuffMage (Game|GetGameMode)))
  (Default|BindTOEnemy (Variables|/Game/Blueprint/Core/GameModes/GM_BuffMage.GM_BuffMage_C|GetRangedSwarmBrain _asgm_buff_mage) self))

(event Collision|EventActorBeginOverlap
  (params (OtherActor :type Actor%20Object%20Reference))
  (|CallParentFunction OtherActor) ; This node is disabled and will not be called.\nDrag off pins to build functionality.
)

(event EventTick
  (params (DeltaSeconds :type Float%20%28single-precision%29))
  (|CallParentFunction DeltaSeconds) ; This node is disabled and will not be called.\nDrag off pins to build functionality.
)

(fn ConstructionScript
  (|CallParentFunction))