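; Base enemy Blueprint that starts its AI behavior tree and provides a basic area attack.
; BeginPlay randomizes EQS ring values, sets the tree on BP_EnemyController and hands its Blackboard to EnemyAttack; the EQS Blackboard writes are disconnected.
; Hp stun and recovery events toggle the bIsStunned Blackboard key.
; AttackSequenceFunction damages pawns in a sphere around AttackOverlapPoint, excluding itself.
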(event Custom|Stunned_Event
  (if (not (ScalableFloat|GetValueasBool (Variables|Default|GetBlackBoard) (Utilities|Name|MakeLiteralName "bIsStunned")))
    (AI|Components|Blackboard|SetValueasBool (Variables|Default|GetBlackBoard) (Utilities|Name|MakeLiteralName "bIsStunned") true)))

(event Custom|StunRecovery_Event
  (AI|Components|Blackboard|SetValueasBool (Variables|Default|GetBlackBoard) (Utilities|Name|MakeLiteralName "bIsStunned") false))

(event EventBeginPlay
  (Utilities|FlowControl|Sequence
    (:then_0
      (Variables|Eqs|points|SetPointsEqs (Math|Random|RandomIntegerinRange (Variables|Eqs|points|GetMinPointsEqs) (Variables|Eqs|points|GetMaxPointsEqs)))
      (Variables|Eqs|Range|SetRangeEqs (Math|Random|RandomFloatinRange (Variables|Eqs|Range|GetMixRangeEqs) (Variables|Eqs|Range|GetMaxRangeEqs)))
      (Variables|Eqs|SetDistanceBetweenPointsEqs (+ (/ (* (Variables|Eqs|Range|GetRangeEqs) 2.0 (Math|Trig|GetPI)) (Math|Conversions|ToFloat(Integer) (Variables|Eqs|points|GetPointsEqs))) 1e+01)))
    (:then_1
      (bind _asbp_enemy_controller (Utilities|Casting|CastToBP_EnemyController (Pawn|GetController)))
      (Default|SetBehaviorTree _asbp_enemy_controller (Variables|Default|GetBTAsset))
      (bind _output_get (Variables|Default|SetBlackBoard (AI|GetBlackboard _asbp_enemy_controller)))
      (Variables|/Game/Blueprint/ActorComponents/BP_EnemyAttack.BP_EnemyAttack_C|SetBlackboard (Variables|Default|GetEnemyAttack) _output_get))
    (:then_2
      (EventDispatchers|BindEventtoOnStunned (Variables|Default|GetHp) (EventDispatchers|CreateEvent :!event Custom|Stunned_Event))
      (EventDispatchers|BindEventtoOnStunRecovered (Variables|Default|GetHp) (EventDispatchers|CreateEvent :!event Custom|StunRecovery_Event)))))

(event Collision|EventActorBeginOverlap
  (params (OtherActor :type Actor%20Object%20Reference)))

(event EventTick
  (params (DeltaSeconds :type Float%20%28single-precision%29)))

(fn ConstructionScript)

(fn AttackSequenceFunction
  (params (SphereRadius :type Float%20%28single-precision%29))
  (bind _outactors (Collision|SphereOverlapActors (Transformation|GetWorldLocation (Variables|Default|GetAttackOverlapPoint)) SphereRadius (Utilities|Array|MakeArray "ObjectTypeQuery3") 0 (Utilities|Array|MakeArray self)))
  (for _array_element _outactors
    (bind _returnvalue (Game|Damage|ApplyDamage _array_element 1.0 0 0))
    (Development|PrintString (Utilities|String|Append "damage dealt = " (Utilities|String|ToString(Float) _returnvalue)))))