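; BP_BuffMage is the player character, wiring attack, health and dash components to UI, weapon switching, pausing and death.
; BeginPlay pools projectiles, sets up controller UI and selects the first weapon; death opens a menu and freezes time.
; Attacks and damage trigger delayed hit stop, with camera shake when hurt.
; Construction adds dynamic post-process materials to the camera for dash and low-health effects; debug keys toggle invincibility and rage or reload behavior.
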(event OnAttackHitDel(AttackComp)
  (Utilities|FlowControl|Sequence
    (:then_0
      (Utilities|FlowControl|Delay 0.2)
      (Class|HitStopComponent|ActivateHitStun (Variables|Default|GetHitStop) 0.0))))

(event OnHit(HpComponent)
  (Utilities|FlowControl|Sequence
    (:then_0
      (Utilities|FlowControl|Delay 0.2)
      (Class|HitStopComponent|ActivateHitStun (Variables|Default|GetHitStop) 0.0))
    (:then_1
      (CameraShakes|StartCameraShake (Game|GetPlayerCameraManager 0) "/Game/Blueprint/Character/CameraShake/BP_CamShakeHit.BP_CamShakeHit_C" 1.0 "CameraLocal" "0, 0, 0"))
    (:then_2
      (CallFunction|PostProcessHit))))

(event OnDeathStarted(HpComponent)
  (bind _returnvalue (UserInterface|CreateWidget "/Game/Blueprint/UI/WBP_DeadMenu.WBP_DeadMenu_C"))
  (UserInterface|Viewport|AddtoViewport _returnvalue 0)
  (Input|SetInputModeUIOnly (Game|GetPlayerController 0) _returnvalue "DoNotLock" false)
  (Utilities|Time|SetGlobalTimeDilation 0.0))

(event OnDeathEnd(HpComponent))

(event OnDashPerformed(DashComponent)
  (Rendering|Material|SetScalarParameterValue (Variables|Default|GetM_PP_DashDynamic) "Alpha" 1.0 :!class /Script/Engine.MaterialInstanceDynamic))

(event OnDashEnded(DashComponent)
  (Rendering|Material|SetScalarParameterValue (Variables|Default|GetM_PP_DashDynamic) "Alpha" 0.0 :!class /Script/Engine.MaterialInstanceDynamic))

(event Input|EnhancedActionEvents|EnhancedInputActionIA_1
  (params (ActionValue :type Boolean) (ElapsedSeconds :type Float%20%28double-precision%29) (TriggeredSeconds :type Float%20%28double-precision%29) (InputAction :type Input%20Action%20Object%20Reference :default "/Game/Blueprint/Character/Inputs/InputActions/IA_1.IA_1"))
  (:Started
    (Class|AttackComponent|SetWeapon (Variables|Default|GetAttackComp))))

(event Input|EnhancedActionEvents|EnhancedInputActionIA_2
  (params (ActionValue :type Boolean) (ElapsedSeconds :type Float%20%28double-precision%29) (TriggeredSeconds :type Float%20%28double-precision%29) (InputAction :type Input%20Action%20Object%20Reference :default "/Game/Blueprint/Character/Inputs/InputActions/IA_2.IA_2"))
  (:Started
    (Class|AttackComponent|SetWeapon (Variables|Default|GetAttackComp) 1)))

(event Input|EnhancedActionEvents|EnhancedInputActionIA_3
  (params (ActionValue :type Boolean) (ElapsedSeconds :type Float%20%28double-precision%29) (TriggeredSeconds :type Float%20%28double-precision%29) (InputAction :type Input%20Action%20Object%20Reference :default "/Game/Blueprint/Character/Inputs/InputActions/IA_3.IA_3"))
  (:Started
    (Class|AttackComponent|SetWeapon (Variables|Default|GetAttackComp) 2)))

(event EventBeginPlay
  (bind _hpcomponent (Variables|Default|GetHpComponent))
  (|CallParentFunction)
  (Class|ObjectPoolingSubsystem|AddPool (Subsystems|GetObjectPoolingSubsystem) "/Game/Testing(TODELETE)/BP_Projectile.BP_Projectile_C" 50)
  (bind _asbp_buff_mage_controller (Utilities|Casting|CastToBP_BuffMageController (Pawn|GetController)))
  (Default|SetupUiValues _asbp_buff_mage_controller self)
  (Class|AttackComponent|ChangeWeapon (Variables|Default|GetAttackComp))
  (Default|CallOnHpChanged _hpcomponent (Variables|/Script/BuffMage.HpComponent|GetCurrentHp _hpcomponent))
  (Rendering|Material|SetScalarParameterValue (Variables|Default|GetM_PP_DamageDynamic) "Alpha" 0.0 :!class /Script/Engine.MaterialInstanceDynamic)
  (Rendering|Material|SetScalarParameterValue (Variables|Default|GetM_PP_DashDynamic) "Alpha" 0.0 :!class /Script/Engine.MaterialInstanceDynamic))

(event EventPauseFunction
  (params (InputActionValue :type Input%20Action%20Value%20Structure%20%28by%20ref%29))
  (if (Variables|Default|GetIsGamePaused)
    (bind _output_get (Variables|Default|SetIsGamePaused false))
    (Game|SetGamePaused _output_get)
    (Widget|RemovefromParent (Variables|Default|GetPauseMenu))
    (Input|SetInputModeGameOnly (Game|GetPlayerController 0) false)
    (else
      (bind _output_get_2 (Variables|Default|SetIsGamePaused true))
      (Game|SetGamePaused _output_get_2)
      (bind _returnvalue (UserInterface|CreateWidget "/Game/Blueprint/UI/WBP_PauseMenu.WBP_PauseMenu_C" (Game|GetPlayerController 0)))
      (bind _output_get_3 (Variables|Default|SetPauseMenu _returnvalue))
      (UserInterface|Viewport|AddtoViewport _output_get_3 0)
      (Input|SetInputModeUIOnly (Game|GetPlayerController 0) (Variables|Default|GetPauseMenu) "LockInFullscreen" false))))

(event EventTick
  (params (DeltaSeconds :type Float%20%28single-precision%29)))

(event Input|KeyboardEvents|DebugKeyU
  (params (Key :type Key%20Structure :default "None") (ActionValue :type Input%20Action%20Value%20Structure))
  (bind _attackcomp (Variables|Default|GetAttackComp))
  ;[0.15 0.00584 0.02043 0.5 174] DEBUG DELETE THIS
  (:Pressed
    (Class|AttackComponent|SetRage _attackcomp 0.0)
    (Class|AttackComponent|StopRage _attackcomp)))

(event Input|KeyboardEvents|DebugKeyT
  (params (Key :type Key%20Structure :default "None") (ActionValue :type Input%20Action%20Value%20Structure))
  ;[0.15 0.00584 0.02043 0.5 174] DEBUG DELETE THIS
  ;;[0.15 0.15 0.15 0.5] Become invincible
  (:Pressed
    (Utilities|FlowControl|FlipFlop
      (:A
        (Components|Activation|Deactivate (Variables|Default|GetHpComponent))
        (Development|PrintString "I'm Invicncible"))
      (:B
        (Components|Activation|Activate (Variables|Default|GetHpComponent) false)
        (Development|PrintString "I'm vincible")))))

(event Input|KeyboardEvents|DebugKeyE
  (params (Key :type Key%20Structure :default "None") (ActionValue :type Input%20Action%20Value%20Structure))
  ;[0.15 0.00584 0.02043 0.5 174] DEBUG DELETE THIS
  ;;[0.15 0.15 0.15 0.5] Stunn all enemies
)

(event Input|KeyboardEvents|DebugKeyL
  (params (Key :type Key%20Structure :default "None") (ActionValue :type Input%20Action%20Value%20Structure))
  ;[0.15 0.00584 0.02043 0.5 174] DEBUG DELETE THIS
  (:Pressed
    (bind _isa (Utilities|FlowControl|FlipFlop)
      (:A
        _)
      (:B
        _))
    (Development|PrintString (Utilities|String|Append "Remove Rage when stopped is " (Utilities|String|ToString(Boolean) _isa)))
    (Variables|/Script/BuffMage.AttackComponent|SetbRemoveRageWhenStopped (Variables|Default|GetAttackComp) _isa)))

(event Input|KeyboardEvents|DebugKey4
  (params (Key :type Key%20Structure :default "None") (ActionValue :type Input%20Action%20Value%20Structure))
  ;[0.15 0.00584 0.02043 0.5 174] DEBUG DELETE THIS
  (:Pressed
    (bind _isa (Utilities|FlowControl|FlipFlop)
      (:A
        _)
      (:B
        _))
    (Development|PrintString (Utilities|String|Append "Reload when ammo finished is " (Utilities|String|ToString(Boolean) (not _isa))))
    (Variables|/Script/BuffMage.AttackComponent|SetbReloadWhenAmmoFinished (Variables|Default|GetAttackComp) (not _isa))))

(event Input|KeyboardEvents|DebugKey5
  (params (Key :type Key%20Structure :default "None") (ActionValue :type Input%20Action%20Value%20Structure))
  ;[0.15 0.00584 0.02043 0.5 174] DEBUG DELETE THIS
  (:Pressed
    (Development|PrintString "FillRage")
    (Class|AttackComponent|AddRage (Variables|Default|GetAttackComp) 1e+03)))

(fn ConstructionScript
  (Variables|/Script/BuffMage.HitStopComponent|SetSceneComponent (Variables|Default|GetHitStop) (Variables|Default|GetCameraComponent))
  (bind _returnvalue (Rendering|Material|CreateDynamicMaterialInstance "/Game/Materials/PostProcess/M_PP_Damage_Inst.M_PP_Damage_Inst" "None" "None" :!class /Script/Engine.KismetMaterialLibrary))
  (Variables|Default|SetM_PP_DamageDynamic _returnvalue)
  (bind _returnvalue_2 (Rendering|Material|CreateDynamicMaterialInstance "/Game/Materials/PostProcess/Dash/M_PP_DashVFX.M_PP_DashVFX" "None" "None" :!class /Script/Engine.KismetMaterialLibrary))
  (Variables|Default|SetM_PP_DashDynamic _returnvalue_2)
  (Utilities|Struct|SetmembersinPostProcessSettings (Variables|/Script/Engine.CameraComponent|GetPostProcessSettings (Variables|Default|GetCameraComponent)) (Utilities|Struct|MakeWeightedBlendables (Utilities|Array|MakeArray (Utilities|Struct|MakeWeightedBlendable 1.0 (Variables|Default|GetM_PP_DashDynamic)) (Utilities|Struct|MakeWeightedBlendable 1.0 (Variables|Default|GetM_PP_DamageDynamic))))))

(fn PlaySound
  (params (Sound :type Sound%20Base%20Object%20Reference) (StartTime :type Float%20%28single-precision%29))
  (Audio|PlaySoundatLocation Sound (Transformation|GetActorLocation) "0, 0, 0" (Math|Random|RandomFloatinRange 0.03 0.05) (Math|Random|RandomFloatinRange 0.7 1.3) StartTime 0 0 0 0))

(fn PlayRandSound
  (params (Sound :type Array%20of%20Sound%20Base%20Object%20References) (StartTime :type Float%20%28single-precision%29))
  (CallFunction|PlaySound (.OutItem (Utilities|Array|Random Sound)) StartTime))

(fn PostProcessHit
  (bind _hpcomponent (Variables|Default|GetHpComponent))
  (bind _output_get (LocalVariables|SetHpPercent (/ (Variables|/Script/BuffMage.HpComponent|GetCurrentHp _hpcomponent) (Variables|/Script/BuffMage.HpComponent|GetMaxHp _hpcomponent))))
  (if (<= _output_get (Variables|PostProcess|GetPercentHpTreshold))
    ;[0.15 0.15 0.15 0.5] Set Radious lerped from 100% to 99.9%
    (Rendering|Material|SetScalarParameterValue (Variables|Default|GetM_PP_DamageDynamic) "Radious" (Math|Float|Lerp (Variables|PostProcess|GetPercentMin) (Variables|PostProcess|GetPercentMax) (/ (LocalVariables|GetHpPercent) (Variables|PostProcess|GetPercentHpTreshold))) :!class /Script/Engine.MaterialInstanceDynamic)
    ;[0.15 0.15 0.15 0.5] Activate Effect
    (Rendering|Material|SetScalarParameterValue (Variables|Default|GetM_PP_DamageDynamic) "Alpha" 0.5 :!class /Script/Engine.MaterialInstanceDynamic)
    (else
      ;[0.15 0.15 0.15 0.5] Deactivate effect
      (Rendering|Material|SetScalarParameterValue (Variables|Default|GetM_PP_DamageDynamic) "Alpha" 0.0 :!class /Script/Engine.MaterialInstanceDynamic))))