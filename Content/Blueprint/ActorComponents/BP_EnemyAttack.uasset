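; Enemy attack component that extends a parent attack component and mirrors its combat state into the AI Blackboard.
; Overridden attack, reload and cooldown events call the parent, set IsAttacking and IsReloading keys, and fire attack start/end dispatchers.
; IsAttacking stays true through the weapon's between-combo cooldown, and depleted ammo triggers reloading.
; Taking damage immediately completes a reload and clears both flags, a stopgap against interrupted reloads.
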(event EventBeginPlay
  (bind _returnvalue (Components|GetOwner))
  (bind _returnvalue_2 (AI|GetBlackboard _returnvalue))
  (|CallParentFunction)
  (Utilities|IsValid (Variables|Default|GetBlackboard)
    (:Is%20Valid
      _)
    (:Is%20Not%20Valid
      (Utilities|IsValid _returnvalue_2
        (:Is%20Valid
          (Variables|Default|SetBlackboard _returnvalue_2)))))
  (CallFunction|SetIsReloading false)
  (CallFunction|SetIsAttacking false))

(event EventReduceAmmo
  (|CallParentFunction))

(event EventAddtoRageAfterKill
  (|CallParentFunction))

(event EventAttackCanbeUsedAgain
  ;[0.15 0.15 0.15 0.5] Should be moved to attack complete if we want to make enemies do combos
  (Default|CallOnAttackEnded)
  (CallFunction|SetIsAttacking false)
  (|CallParentFunction))

(event EventOnDamageReceived
  (params (Actor :type Actor%20Object%20Reference) (X :type Float%20%28single-precision%29) (Damage :type Damage%20Type%20Object%20Reference) (Controller :type Controller%20Object%20Reference) (Actor1 :type Actor%20Object%20Reference))
  (|CallParentFunction Actor X Damage Controller Actor1)
  ;[0.15 0.15 0.15 0.5] Here cause if you interrupt enemy while reloading it will never reload
  ; (nned to change tho)
  (Class|AttackComponent|ReloadWeapon)
  (CallFunction|SetIsReloading false)
  (CallFunction|SetIsAttacking false))

(event EventStartRage
  (|CallParentFunction))

(event EventStopRage
  (|CallParentFunction))

(event EventTick
  (params (DeltaSeconds :type Float%20%28single-precision%29))
  (|CallParentFunction 0.0))

(event EventSetCooldownTime
  (|CallParentFunction)
  (CallFunction|SetIsAttacking true)
  (Utilities|FlowControl|Delay (Variables|/Script/BuffMage.WeaponDataAsset|GetCooldownBetweenCombos (Utilities|Struct|BreakDynamicWeaponData (Variables|Default|GetCurrentWeapon))))
  (CallFunction|SetIsAttacking false))

(event EventStartReloading
  (|CallParentFunction)
  (CallFunction|SetIsReloading true)
  (CallFunction|SetIsAttacking false))

(event EventAttackCompleted
  (CallFunction|SetIsAttacking false)
  (|CallParentFunction))

(event EventChangeWeapon
  (params (InputValue :type Integer))
  (|CallParentFunction InputValue))

(event EventHitDetection
  (params (SocketName :type Name :default "None"))
  (|CallParentFunction SocketName))

(event EventReloadWeapon
  (Default|CallOnAttackEnded)
  (CallFunction|SetIsReloading false)
  (|CallParentFunction))

(event EventStartAttackAnim
  (Default|CallOnAttackStart)
  (CallFunction|SetIsAttacking true)
  (|CallParentFunction))

(event EventAddRage
  (params (Amount :type Float%20%28single-precision%29))
  (|CallParentFunction Amount))

(fn SetIsReloading
  (params (Value :type Boolean))
  (Utilities|IsValid (Variables|Default|GetBlackboard)
    (:Is%20Valid
      (AI|Components|Blackboard|SetValueasBool (Variables|Default|GetBlackboard) (Utilities|Name|MakeLiteralName "IsReloading") Value))))

(fn UpdateAttackSpeed)

(fn SetIsAttacking
  (params (Value :type Boolean))
  (Utilities|IsValid (Variables|Default|GetBlackboard)
    (:Is%20Valid
      (AI|Components|Blackboard|SetValueasBool (Variables|Default|GetBlackboard) (Utilities|Name|MakeLiteralName "IsAttacking") Value))))

(fn HasAmmoBeenDepleted
  (bind _returnvalue (|CallParentFunction))
  (if _returnvalue
    (Class|AttackComponent|StartReloading))
  (return _returnvalue))

(fn GetBlackboard
  (params (Blackboard :type Blackboard%20Component%20Object%20Reference))
  (Variables|Default|SetBlackboard Blackboard)
  (CallFunction|SetIsReloading false)
  (CallFunction|SetIsAttacking false))

(fn GetBoolfromBlackboard
  (params (KeyName :type Name%20%28by%20ref%29))
  (return (ScalableFloat|GetValueasBool (Variables|Default|GetBlackboard) KeyName)))