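; Player controller for the Buff Mage that owns the game HUD, dialogue and checkpoint-return widgets.
; SetupUiValues binds a target's Attack, HP and Dash component events to handlers that push ammo, weapon icon, rage, health, shield and dash into the GameUI.
; Dialogue system events show and hide the dialogue widget.
; It also stores the latest checkpoint and disables input during the checkpoint fade.
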(event Custom|StartDialogueEvent
  (params (Dialogue :type Dialogue%20Structure))
  (UserInterface|Viewport|AddtoViewport (Variables|Default|GetDialogueUI) 0)
  (Default|OnDialogueStart (Variables|Default|GetDialogueUI) Dialogue))

(event Custom|OnDialogueEndedEvent
  (Widget|RemovefromParent (Variables|Default|GetDialogueUI))
  (Default|ChangeBuffMageExpression (Variables|Default|GetGameUI) "/Game/Blueprint/UI/Test_Images/IMG_Base.IMG_Base"))

(event Custom|OnFadeEnded_Event
  (Widget|RemovefromParent (Variables|Default|GetCheckPointUI))
  (Input|EnableInput self))

(event Custom|StartFade
  (UserInterface|Viewport|AddtoViewport (Variables|Default|GetCheckPointUI) 0)
  (Input|DisableInput self))

(event Custom|BindToCheckpoints
  (params (CheckPoint :type BP%20Check%20Point%20Lava%20Object%20Reference))
  (EventDispatchers|AssignOnPlayerNewCheckPoint CheckPoint (EventDispatchers|CreateEvent :!event Custom|OnNewCheckpoint)))

(event Custom|OnNewCheckpoint
  (params (NewCheckpointPos :type Vector))
  (Variables|Default|SetCurrentCheckpoint NewCheckpointPos))

(event EventBeginPlay
  (Variables|Default|SetbShowMouseCursor false)
  (EventDispatchers|BindEventtoOnStartDialogue (Subsystems|GetDialogueSystem) (EventDispatchers|CreateEvent :!event Custom|StartDialogueEvent))
  (bind _returnvalue (UserInterface|CreateWidget "/Game/Blueprint/UI/WBP_DialogueUI.WBP_DialogueUI_C"))
  (bind _output_get (Variables|Default|SetDialogueUI _returnvalue))
  (EventDispatchers|BindEventtoOnDialogueEnd _output_get (EventDispatchers|CreateEvent :!event Custom|OnDialogueEndedEvent))
  (bind _returnvalue_2 (UserInterface|CreateWidget "/Game/Blueprint/UI/WBP_GameUI.WBP_GameUI_C"))
  (bind _output_get_2 (Variables|Default|SetGameUI _returnvalue_2))
  (UserInterface|Viewport|AddtoViewport _output_get_2 0)
  (Input|SetInputModeGameOnly self false)
  (bind _returnvalue_3 (UserInterface|CreateWidget "/Game/Blueprint/UI/WBP_ReturnToCheckPoint.WBP_ReturnToCheckPoint_C"))
  (Variables|Default|SetCheckPointUI _returnvalue_3)
  (Class|EnhancedInputSubsystemInterface|SetInputMode(Message) self (Utilities|Struct|MakeGameplayTagContainer (Utilities|Array|MakeArray "(TagName=\"UI\")" "(TagName=\"EnhancedInput\")"))))

(event EventTick
  (params (DeltaSeconds :type Float%20%28single-precision%29)))

(fn ConstructionScript)

(fn SetupUiValues
  (params (Target :type Actor%20Object%20Reference))
  (Utilities|FlowControl|Sequence
    (:then_0
      (LocalVariables|SetAttackComp (Actor|GetComponentbyClass Target "/Script/BuffMage.AttackComponent"))
      (EventDispatchers|BindEventtoOnAmmoChange (LocalVariables|GetAttackComp) (EventDispatchers|CreateEvent :!event OnPlayerAmmoChanged))
      (EventDispatchers|BindEventtoOnWeaponIconChanged (LocalVariables|GetAttackComp) (EventDispatchers|CreateEvent :!event OnPlayerWeaponIconChanged))
      (EventDispatchers|BindEventtoOnRageChange (LocalVariables|GetAttackComp) (EventDispatchers|CreateEvent :!event OnPlayerRageChange))
      (EventDispatchers|BindEventtoOnActivatingRage (LocalVariables|GetAttackComp) (EventDispatchers|CreateEvent :!event OnPlayerRageActivation))
      (EventDispatchers|BindEventtoOnDeactivatingRage (LocalVariables|GetAttackComp) (EventDispatchers|CreateEvent :!event OnPlayerRageDeactivation)))
    (:then_1
      (LocalVariables|SetHpComponent (Actor|GetComponentbyClass Target "/Script/BuffMage.HpComponent"))
      (EventDispatchers|BindEventtoOnHpChanged (LocalVariables|GetHpComponent) (EventDispatchers|CreateEvent :!event OnPlayerHpChanged))
      (EventDispatchers|BindEventtoOnShieldChanged (LocalVariables|GetHpComponent) (EventDispatchers|CreateEvent :!event OnPlayerShieldChanged)))
    (:then_2
      (LocalVariables|SetDashComp (Actor|GetComponentbyClass Target "/Script/BuffMage.DashComponent"))
      (EventDispatchers|BindEventtoOnDashChange (LocalVariables|GetDashComp) (EventDispatchers|CreateEvent :!event OnPlayerDashChange)))
    (:then_3
      (EventDispatchers|BindEventtoOnFadeCompleted (Variables|Default|GetCheckPointUI) (EventDispatchers|CreateEvent :!event Custom|OnFadeEnded_Event)))))

(fn OnPlayerAmmoChanged
  (params (CurrentAmount :type Float%20%28single-precision%29))
  (Default|ChangeAmmoValue (Variables|Default|GetGameUI) (Utilities|Text|ToText(Float) CurrentAmount "HalfToEven")))

(fn OnPlayerWeaponIconChanged
  (params (Icon :type Texture%202D%20Soft%20Object%20Reference))
  (Default|ChangeWeaponIcon (Variables|Default|GetGameUI) Icon))

(fn OnPlayerRageChange
  (params (CurrentAmount :type Float%20%28single-precision%29) (MaximumAmount :type Float%20%28single-precision%29))
  (Default|ChangeRageBar (Variables|Default|GetGameUI) (/ CurrentAmount MaximumAmount)))

(fn OnPlayerHpChanged
  (params (CurrentHp :type Float%20%28single-precision%29))
  (Default|ChangeHpValue (Variables|Default|GetGameUI) (Utilities|Text|ToText(Float) CurrentHp "HalfToEven")))

(fn OnPlayerRageActivation
  ;[0.15 0.15 0.15 0.5] Debug needs to change
  (Default|OnRageActivation (Variables|Default|GetGameUI)))

(fn OnPlayerRageDeactivation
  ;[0.15 0.15 0.15 0.5] Debug needs to change
  (Default|OnRageDeactivation (Variables|Default|GetGameUI)))

(fn OnPlayerDashChange
  (params (CurrentAmount :type Float%20%28single-precision%29) (MaxAmount :type Float%20%28single-precision%29))
  (Default|SetDashPercentage (Variables|Default|GetGameUI) (/ CurrentAmount MaxAmount)))

(fn OnPlayerShieldChanged
  (params (CurrentHp :type Float%20%28single-precision%29))
  (Default|ChangeShieldValue (Variables|Default|GetGameUI) (Utilities|Text|ToText(Float) CurrentHp "HalfToEven")))