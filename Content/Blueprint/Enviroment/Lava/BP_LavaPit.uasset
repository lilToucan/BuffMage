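; BP_LavaPit is a lava hazard that damages actors with an HpComponent when they begin overlapping its Cube.
; The first player pawn takes damage directly through HpComponent's ApplyDamageDirectly with fade enabled, while other such actors receive standard ApplyDamage.
; Damage is applied once per overlap begin, and a disconnected SetActorLocation teleport node never runs.
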(event OnComponentBeginOverlap(Cube)
  (params (OverlappedComponent :type Primitive%20Component%20Object%20Reference) (OtherActor :type Actor%20Object%20Reference) (OtherComp :type Primitive%20Component%20Object%20Reference) (OtherBodyIndex :type Integer) (bFromSweep :type Boolean) (SweepResult :type Hit%20Result%20Structure%20%28by%20ref%29))
  (bind _returnvalue (Actor|GetComponentbyClass OtherActor "/Script/BuffMage.HpComponent"))
  (Utilities|IsValid _returnvalue
    (:Is%20Valid
      (if (== (Components|GetOwner _returnvalue) (Game|Player|GetPlayerPawn 0))
        (Class|HpComponent|ApplyDamageDirectly _returnvalue 0 (Variables|Default|GetDanage) 0 0 self true)
        (else
          (Game|Damage|ApplyDamage OtherActor (Variables|Default|GetDanage) 0 self))))))

(fn ConstructionScript)