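; BP_Lever is an environment lever that only a player of class BP_BuffMage can use.
; On Interact, it calls OnKeyUnLock on its Key reference and plays a timeline from the start.
; The timeline linearly interpolates the Handle's world location from StartingPoint to EndingPoint and clears IsUsable as it updates, so the lever works once.
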(event EventInteract
  (params (Player :type Buff%20Mage%20Character%20Object%20Reference))
  (bind _startingpoint (Variables|Default|GetStartingPoint))
  (bind _returnvalue (Transformation|GetWorldLocation _startingpoint))
  (if (== (Utilities|GetClass Player) "/Game/Blueprint/Character/BP_BuffMage.BP_BuffMage_C")
    (if (Variables|Default|GetIsUsable)
      (Default|CallOnKeyUnLock (Variables|Default|GetKey))
      (bind _elevatormoving (Timeline|Timeline PlayFromStart)
        (:Update
          (Transformation|SetWorldLocation (Variables|Default|GetHandle) (+ (* _elevatormoving (- (Transformation|GetWorldLocation (Variables|Default|GetEndingPoint)) _returnvalue)) _returnvalue) false false)
          (Variables|Default|SetIsUsable false))))))

(fn ConstructionScript)