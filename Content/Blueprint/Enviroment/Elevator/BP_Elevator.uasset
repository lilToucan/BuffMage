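; BP_Elevator is an elevator that moves when a BP_BuffMage overlaps its trigger.
; The overlap plays the ElevatorMoving timeline, which interpolates the Elevator component's world location from StartingPoint to EndingPoint without sweeping.
; An IsMoving flag is set during timeline updates to block retriggering and is never cleared here, so the graph provides a one-way, single-use ride.
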(event OnComponentBeginOverlap(Trigger)
  (params (OverlappedComponent :type Primitive%20Component%20Object%20Reference) (OtherActor :type Actor%20Object%20Reference) (OtherComp :type Primitive%20Component%20Object%20Reference) (OtherBodyIndex :type Integer) (bFromSweep :type Boolean) (SweepResult :type Hit%20Result%20Structure%20%28by%20ref%29))
  (bind _startingpoint (Variables|Default|GetStartingPoint))
  (bind _returnvalue (Transformation|GetWorldLocation _startingpoint))
  (if (== (Utilities|GetClass OtherActor) "/Game/Blueprint/Character/BP_BuffMage.BP_BuffMage_C")
    (if (not (Variables|Default|GetIsMoving))
      (bind _elevatormoving (Timeline|Elevator%20Moving Play)
        (:Update
          (Transformation|SetWorldLocation (Variables|Default|GetElevator) (+ (* _elevatormoving (- (Transformation|GetWorldLocation (Variables|Default|GetEndingPoint)) _returnvalue)) _returnvalue) false false)
          (Variables|Default|SetIsMoving true))))))

(fn ConstructionScript)