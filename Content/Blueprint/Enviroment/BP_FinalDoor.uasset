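; BP_FinalDoor is a sliding door that opens when something overlaps its Box trigger while it is unlocked.
; The Lock's OnLocked and OnUnLocked events set IsUnlocked, which gates the overlap.
; A Timeline scaled to Duration lerps the Door's relative location between the Closed and Open component positions.
; Nothing closes the door, and the OpentheDoor and ClosetheDoor events are empty.
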(event OnLocked(Lock)
  (Variables|Default|SetIsUnlocked false))

(event OnUnLocked(Lock)
  (Variables|Default|SetIsUnlocked true))

(event OnComponentBeginOverlap(Box)
  (params (OverlappedComponent :type Primitive%20Component%20Object%20Reference) (OtherActor :type Actor%20Object%20Reference) (OtherComp :type Primitive%20Component%20Object%20Reference) (OtherBodyIndex :type Integer) (bFromSweep :type Boolean) (SweepResult :type Hit%20Result%20Structure%20%28by%20ref%29))
  (if (Variables|Default|GetIsUnlocked)
    (Components|Timeline|SetPlayRate (Variables|Default|GetTimeline) (/ 1.0 (Variables|Default|GetDuration)))
    (bind _opendoor (Timeline|Timeline Play)
      (:Update
        (Transformation|SetRelativeLocation (Variables|Default|GetDoor) (Math|Vector|Lerp(Vector) (Variables|/Script/Engine.SceneComponent|GetRelativeLocation (Variables|Default|GetClosed)) (Variables|/Script/Engine.SceneComponent|GetRelativeLocation (Variables|Default|GetOpen)) _opendoor) false false)))))

(event EventOpentheDoor)

(event EventClosetheDoor)

(fn ConstructionScript
  (|CallParentFunction))