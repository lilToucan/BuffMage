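; Pooled projectile actor that damages what it overlaps, ignoring other projectiles of its class, its shooter, and enemies when an enemy fired it.
; Activate stores shot parameters, positions and enables the actor, then launches it forward through ProjectileMovement.
; A valid overlap applies damage and calls Deactivate, which hides the actor, stops it and returns it to the ObjectPoolingSubsystem.
; ExplosionRange is stored but never used here.
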(event EventBeginPlay)

(event EventTick
  (params (DeltaSeconds :type Float%20%28single-precision%29)))

(event EventActivate
  (params (Velocity :type Float%20%28single-precision%29) (Damage :type Float%20%28single-precision%29) (ExplosionRange :type Float%20%28single-precision%29) (Shooter :type Actor%20Object%20Reference) (Position :type Vector :default "0, 0, 0") (Rotation :type Rotator :default "0, 0, 0"))
  (Variables|Default|SetVelocity Velocity)
  (Variables|Default|SetDamage Damage)
  (Variables|Default|SetExplosion%20Range ExplosionRange)
  (Variables|Default|SetShooter Shooter)
  (Transformation|SetActorLocation Position false false)
  (Transformation|SetActorRotation Rotation)
  (Actor|Tick|SetActorTickEnabled true)
  (Rendering|SetActorHiddenInGame false)
  (Collision|SetActorEnableCollision true)
  (Variables|/Script/Engine.MovementComponent|SetVelocity (Variables|Default|GetProjectileMovement) (* (Transformation|GetActorForwardVector) (Variables|Default|GetVelocity))))

(event EventDeactivate
  (Rendering|SetActorHiddenInGame true)
  (Collision|SetActorEnableCollision false)
  (Actor|Tick|SetActorTickEnabled false)
  (Class|ObjectPoolingSubsystem|ReturnActortoPool (Subsystems|GetObjectPoolingSubsystem) (Utilities|GetClass self) self)
  (Variables|/Script/Engine.MovementComponent|SetVelocity (Variables|Default|GetProjectileMovement) "0, 0, 0"))

(event Collision|EventActorBeginOverlap
  (params (OtherActor :type Actor%20Object%20Reference))
  (if (not (CallFunction|ColliSionChek OtherActor))
    (Game|Damage|ApplyDamage OtherActor (Variables|Default|GetDamage) 0 (Variables|Default|GetShooter))
    (Class|ProjectilePoolable|Deactivate self)))

(fn ConstructionScript)

(fn ColliSionChek
  (params (HitActor :type Object%20Object%20Reference))
  (return (Math|Boolean|ORBoolean (== (Utilities|GetClass HitActor) (Utilities|GetClass self)) (== HitActor (Variables|Default|GetShooter)) (and (Utilities|ClassIsChildOf (Utilities|GetClass HitActor) "/Game/Blueprint/AI/Enemies/BP_BaseEnemy.BP_BaseEnemy_C") (Utilities|ClassIsChildOf (Utilities|GetClass (Variables|Default|GetShooter)) "/Game/Blueprint/AI/Enemies/BP_BaseEnemy.BP_BaseEnemy_C")))))