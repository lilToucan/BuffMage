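; BP_HealthPack is a test health pack actor that bobs up and down, with no pickup or healing logic.
; Tick accumulates a timer and feeds it to a Sin helper that sets the Sphere component's relative Z.
; The helper offsets the sine wave so the bounce stays between zero and BounceHight.
; BeginPlay, ActorBeginOverlap and the construction script are empty.
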(event EventBeginPlay)

(event Collision|EventActorBeginOverlap
  (params (OtherActor :type Actor%20Object%20Reference)))

(event EventTick
  (params (DeltaSeconds :type Float%20%28single-precision%29))
  (bind _output_get (Variables|Default|SetTimer (+ DeltaSeconds (Variables|Default|GetTimer))))
  (Transformation|SetRelativeLocation (Variables|Default|GetSphere) (Math|Vector|MakeVector 0.0 0.0 (CallFunction|Sin _output_get)) false false))

(fn ConstructionScript)

(fn Sin
  (params (Time :type Float%20%28double-precision%29))
  (return (+ (* (Math|Trig|Sin(Radians) (* Time 3.0)) (/ (Variables|Default|GetBounceHight) 2.0)) (/ (Variables|Default|GetBounceHight) 2.0))))